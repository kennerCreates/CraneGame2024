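; BP_Crane is a drivable crane vehicle pawn that passes player input to its vehicle movement component.
; When a BP_CraneController takes control, it adds the IMC_DriveCrane Enhanced Input mapping context.
; IA_Drive sets steering and throttle, selecting first gear for positive Y and reverse otherwise, with the raw Y as throttle in both cases.
; IA_Brake sets the brake, and releasing either action zeroes its inputs.
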(event `self.ReceiveBeginPlay`)

(event `self.ReceiveControllerChanged`
  (params (OldController :type "Controller Object Reference") (NewController :type "Controller Object Reference"))
  (bind _asbp_crane_controller (cast `/Game/A_Character/Crane/BP_CraneController` NewController))
  (`EnhancedInputSubsystemInterface.AddMappingContext` (pcsubsystem `EnhancedInputLocalPlayerSubsystem` _asbp_crane_controller) "/Game/A_Gameplay/Input/IMC_DriveCrane.IMC_DriveCrane" 0 (struct)))

(event `EnhancedInput|/Game/A_Gameplay/Input/Actions/IA_Drive`
  (params (ActionValue :type "Vector2D Structure") (ElapsedSeconds :type "Float (double-precision)") (TriggeredSeconds :type "Float (double-precision)") (InputAction :type "InputAction Object Reference" :default "/Game/A_Gameplay/Input/Actions/IA_Drive.IA_Drive"))
  (bind _vehiclemovementcomponent (`self.VehicleMovementComponent`))
  (bind _vehiclemovementcomponent_2 (`self.VehicleMovementComponent`))
  (:`Triggered`
    (`ChaosVehicleMovementComponent.SetSteeringInput` (`self.VehicleMovementComponent`) ActionValue_X)
    (if (> ActionValue_Y 0.0)
      (`ChaosVehicleMovementComponent.SetTargetGear` _vehiclemovementcomponent 1 false)
      (`ChaosVehicleMovementComponent.SetThrottleInput` _vehiclemovementcomponent ActionValue_Y)
      (else
        (`ChaosVehicleMovementComponent.SetTargetGear` _vehiclemovementcomponent_2 -1 false)
        (`ChaosVehicleMovementComponent.SetThrottleInput` _vehiclemovementcomponent_2 ActionValue_Y))))
  (:`Completed`
    (`ChaosVehicleMovementComponent.SetSteeringInput` (`self.VehicleMovementComponent`) 0.0)
    (`ChaosVehicleMovementComponent.SetThrottleInput` (`self.VehicleMovementComponent`) 0.0)))

(event `EnhancedInput|/Game/A_Gameplay/Input/Actions/IA_Brake`
  (params (ActionValue :type "Float (double-precision)") (ElapsedSeconds :type "Float (double-precision)") (TriggeredSeconds :type "Float (double-precision)") (InputAction :type "InputAction Object Reference" :default "/Game/A_Gameplay/Input/Actions/IA_Brake.IA_Brake"))
  (:`Triggered`
    (`ChaosVehicleMovementComponent.SetBrakeInput` (`self.VehicleMovementComponent`) ActionValue))
  (:`Completed`
    (`ChaosVehicleMovementComponent.SetBrakeInput` (`self.VehicleMovementComponent`) 0.0)))

(fn `UserConstructionScript`)